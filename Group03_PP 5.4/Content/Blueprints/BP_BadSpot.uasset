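; BP_BadSpot is a hazard actor that kills the player on overlap and teleports them to a respawn point.
; Any overlap first sets the game mode's DeathCount to CoinCount + 1, rather than incrementing DeathCount.
; An EpicCharacter overlap then triggers controller rumble, an explosion effect and sound, and teleports player 0 to RespawnPoint with zero rotation.
; The HUD's UpdateDeaths call is disconnected and never runs.
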(event Collision|EventActorBeginOverlap
  (params (OtherActor :type Actor%20Object%20Reference))
  (bind _asthird_person_game_mode (Utilities|Casting|CastToThirdPersonGameMode (Game|GetGameMode)))
  (Variables|/Game/Blueprints/ThirdPersonGameMode.ThirdPersonGameMode_C|SetdeathCount _asthird_person_game_mode (+ (Variables|/Game/Blueprints/ThirdPersonGameMode.ThirdPersonGameMode_C|GetcoinCount _asthird_person_game_mode) 1))
  (bind _asepic_character (Utilities|Casting|CastToEpicCharacter OtherActor))
  (Game|Feedback|ClientPlayForceFeedback (Game|GetPlayerController 0) "/Game/Assets/ControllerForceFeedback.ControllerForceFeedback" "None" false false false)
  (Effects|SpawnEmitteratLocation "/Game/StarterContent/Particles/P_Explosion.P_Explosion" (Transformation|GetActorLocation _asepic_character))
  (Audio|PlaySound2D "/Game/StarterContent/Audio/Explosion02.Explosion02" 1.0 1.0 0.0 0 0)
  (Transformation|Teleport (Game|GetPlayerCharacter 0) (Transformation|GetActorLocation (Variables|Default|GetRespawnPoint)) "0, 0, 0"))

(fn ConstructionScript)