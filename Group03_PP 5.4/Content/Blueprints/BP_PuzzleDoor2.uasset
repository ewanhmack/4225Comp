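; BP_PuzzleDoor2 is a puzzle door that opens while enough pressure pads are held down.
; SwitchActivated and SwitchDeactivated raise and lower an active pad count, then compare it to the required number.
; The OpenDoor timeline plays when the count is met and reverses otherwise, sliding the Door component along its relative X axis.
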(event Custom|SwitchActivated
  ;[1 1 1] Detecting if plate pushed down
  (Math|Integer|IncrementInt (Variables|Default|GetPressurePadActive)
    (:%20%20
      (if (>= (Variables|Default|GetPressurePadActive) (Variables|Default|GetPressurePadNeeded))
        ;[1 1 1] Door move script
        (bind _doorposition (Timeline|OpenDoor Play)
          (:Update
            (Transformation|SetRelativeLocation (Variables|Default|GetDoor) (Math|Vector|MakeVector _doorposition 0.0 0.0) false false)))
        (else
          (Timeline|OpenDoor Reverse))))))

(event Custom|SwitchDeactivated
  ;[1 1 1] Detect if plate is up
  (Math|Integer|DecrementInt (Variables|Default|GetPressurePadActive)
    (:%20%20
      (if (>= (Variables|Default|GetPressurePadActive) (Variables|Default|GetPressurePadNeeded))
        ;[1 1 1] Door move script
        (bind _doorposition (Timeline|OpenDoor Play)
          (:Update
            (Transformation|SetRelativeLocation (Variables|Default|GetDoor) (Math|Vector|MakeVector _doorposition 0.0 0.0) false false)))
        (else
          (Timeline|OpenDoor Reverse))))))

(fn ConstructionScript)