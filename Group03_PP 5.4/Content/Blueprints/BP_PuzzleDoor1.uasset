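; BP_PuzzleDoor1 is a puzzle door that opens once enough pressure pads are active.
; SwitchActivated and SwitchDeactivated events raise or lower an active pad count and compare it to the required number.
; Meeting that number plays the OpenDoor timeline, which drives the Door's relative Z location, while falling short reverses it.
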(event Custom|SwitchActivated
  (Math|Integer|IncrementInt (Variables|Default|GetPressurePadActive)
    (:%20%20
      (if (>= (Variables|Default|GetPressurePadActive) (Variables|Default|GetPressurePadNeeded))
        (bind _doorposition (Timeline|OpenDoor Play)
          (:Update
            (Transformation|SetRelativeLocation (Variables|Default|GetDoor) (Math|Vector|MakeVector 0.0 0.0 _doorposition) false false)))
        (else
          (Timeline|OpenDoor Reverse))))))

(event Custom|SwitchDeactivated
  (Math|Integer|DecrementInt (Variables|Default|GetPressurePadActive)
    (:%20%20
      (if (>= (Variables|Default|GetPressurePadActive) (Variables|Default|GetPressurePadNeeded))
        (bind _doorposition (Timeline|OpenDoor Play)
          (:Update
            (Transformation|SetRelativeLocation (Variables|Default|GetDoor) (Math|Vector|MakeVector 0.0 0.0 _doorposition) false false)))
        (else
          (Timeline|OpenDoor Reverse))))))

(fn ConstructionScript)